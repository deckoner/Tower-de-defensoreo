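; BP_Torre is a tower that fires a homing projectile at enemies entering its range.
; When a BP_Base_Enemigo begins overlapping RangoTorre, the tower stores it as EnemigoObjetivo and calls Disparar.
; Disparar spawns the Proyectil class at the Billboard's transform and sets its ProjectileMovement homing target to the enemy's capsule.
; Each overlap triggers a single shot, with no timer or repeat fire.
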(event `self.RangoTorre.OnComponentBeginOverlap`
  (params (OverlappedComponent :type "PrimitiveComponent Object Reference") (OtherActor :type "Actor Object Reference") (OtherComp :type "PrimitiveComponent Object Reference") (OtherBodyIndex :type Integer) (bFromSweep :type Boolean) (SweepResult :type "HitResult Structure (by ref)"))
  (bind _asbp_base_enemigo (cast `/Game/Mio/Enemigos/BP_Base_Enemigo` OtherActor))
  (set `self.EnemigoObjetivo` _asbp_base_enemigo)
  (`self.Disparar`))

(fn `Disparar`
  (bind _returnvalue (`|SpawnActorFromClass` (`self.Proyectil`) (`SceneComponent.K2_GetComponentToWorld` (`self.Billboard`)) "Undefined" "MultiplyWithRoot" null null null))
  (set `ProjectileMovementComponent.HomingTargetComponent` (`Character.CapsuleComponent` (`self.EnemigoObjetivo`)) (`/Game/Mio/Torre/BP_Proyectil.ProjectileMovement` _returnvalue)))

(fn `UserConstructionScript`)